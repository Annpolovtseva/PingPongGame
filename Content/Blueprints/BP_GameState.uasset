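; Game state Blueprint that displays the scores of two players in an on-screen widget.
; On BeginPlay, only instances without authority create the W_Score widget and add it to the viewport.
; The UpdateScore event writes the Player 0 and Player 1 scores into that widget's two text fields.
; The score getters and the caller of UpdateScore are defined outside this graph.
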(event `self.ReceiveBeginPlay`
  (`/Engine/EditorBlueprintResources/ActorMacros.Switch Has Authority`
    (:`Remote`
      (bind _returnvalue (`|CreateWidget` "/Game/Blueprints/W_Score.W_Score_C"))
      (bind _output_get (set `self.ScoreWidget` _returnvalue))
      (`UserWidget.AddToViewport` _output_get 0))))

(event `self.UpdateScore`
  (bind _scorewidget (`self.ScoreWidget`))
  (`TextBlock.SetText` (`/Game/Blueprints/W_Score.ScorePlayer1` _scorewidget) (`KismetTextLibrary.Conv_IntToText` (`self.GetPlayer0Score`)))
  (`TextBlock.SetText` (`/Game/Blueprints/W_Score.ScorePlayer2` _scorewidget) (`KismetTextLibrary.Conv_IntToText` (`self.GetPlayer1Score`))))

(fn `UserConstructionScript`)